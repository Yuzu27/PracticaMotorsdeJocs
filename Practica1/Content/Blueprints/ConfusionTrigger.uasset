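; ConfusionTrigger is an overlap trigger actor that inflicts a confusion state on the player character.
; On BeginPlay it finds the ThirdPersonCharacter and caches it as the Player reference.
; When that player overlaps it, it prints a debug message, calls ConfusionState on the player with its ConfusionTime, and destroys itself, so it fires only once.
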(event EventBeginPlay
  (bind _returnvalue (Actor|GetActorOfClass "/Game/ThirdPersonBP/Blueprints/ThirdPersonCharacter.ThirdPersonCharacter_C"))
  (Variables|Default|SetPlayer _returnvalue))

(event Collision|EventActorBeginOverlap
  (params (OtherActor :type Actor%20Object%20Reference))
  (if (== OtherActor (Variables|Default|GetPlayer))
    (Development|PrintString "CONFUSED")
    (Default|ConfusionState (Variables|Default|GetPlayer) (Variables|Default|GetConfusionTime))
    (Actor|DestroyActor)))

(fn ConstructionScript)