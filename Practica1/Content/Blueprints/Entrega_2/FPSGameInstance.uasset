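; Game instance for an FPS that holds coin and key counts, door states and level flow between the main menu and the Landscape level.
; Events collect, spend and reset collectibles, while Play and Restart store a load-checkpoint flag before opening the level.
; Checkpoints save the player transform, collectibles and door flags to one save slot.
; Loading restores them and refreshes the HUD, or saves and then resets collectibles when no save exists.
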(event Custom|CollectCoin
  ;[1 1 1] COLLECTIBLES
  (Variables|Default|SetCoins (+ (Variables|Default|GetCoins) 1)))

(event Custom|CollectKey
  ;[1 1 1] COLLECTIBLES
  (Variables|Default|SetKeys (+ (Variables|Default|GetKeys) 1)))

(event Custom|UseKey
  ;[1 1 1] COLLECTIBLES
  (Variables|Default|SetKeys (- (Variables|Default|GetKeys) 1)))

(event Custom|ResetCollectibles
  ;[1 1 1] COLLECTIBLES
  (Variables|Default|SetKeys 0)
  (Variables|Default|SetCoins 0))

(event Custom|Restart
  (params (LoadCheckpoint :type Boolean))
  (Variables|Default|SetLoadCheckpoint LoadCheckpoint)
  (bind _returnvalue (Game|GetCurrentLevelName true))
  (Game|OpenLevel(byName) (Utilities|String|StringToName _returnvalue)))

(event Custom|ExitToMenu
  (Game|OpenLevel(byName) "MainMenu"))

(event Custom|LoadGame
  (bind _returnvalue (SaveGame|DoesSaveGameExist "SavedGame"))
  (if _returnvalue
    (bind _returnvalue_2 (SaveGame|LoadGamefromSlot "SavedGame"))
    (Transformation|SetActorTransform (Variables|Default|GetPlayer) (Variables|/Game/Blueprints/Entrega_3/Save_Game.Save_Game_C|GetPlayerTransform (.AsSave%20Game (Utilities|Casting|CastToSave_Game _returnvalue_2))))
    (Variables|Default|SetCoins (Variables|/Game/Blueprints/Entrega_3/Save_Game.Save_Game_C|GetCoins (.AsSave%20Game (Utilities|Casting|CastToSave_Game _returnvalue_2))))
    (Variables|Default|SetKeys (Variables|/Game/Blueprints/Entrega_3/Save_Game.Save_Game_C|GetKeys (.AsSave%20Game (Utilities|Casting|CastToSave_Game _returnvalue_2))))
    (Default|UpdateCoins (Variables|/Game/Blueprints/Entrega_2/HUD/HUD_Controller.HUD_Controller_C|GetUI (Variables|Default|GetHUDController)))
    (Default|UpdateKeys (Variables|/Game/Blueprints/Entrega_2/HUD/HUD_Controller.HUD_Controller_C|GetUI (Variables|Default|GetHUDController)))
    (Variables|Default|SetFirstDoorOpened (Variables|/Game/Blueprints/Entrega_3/Save_Game.Save_Game_C|GetFirstDoorOpened (.AsSave%20Game (Utilities|Casting|CastToSave_Game _returnvalue_2))))
    (Variables|Default|SetFinalDoorOpened (Variables|/Game/Blueprints/Entrega_3/Save_Game.Save_Game_C|GetFinalDoorOpened (.AsSave%20Game (Utilities|Casting|CastToSave_Game _returnvalue_2))))
    (else
      (CallFunction|SaveGame)
      (CallFunction|ResetCollectibles))))

(event Custom|Play
  (params (LoadCheckpoint :type Boolean))
  (Variables|Default|SetLoadCheckpoint LoadCheckpoint)
  (Game|OpenLevel(byName) "Landscape"))

(event Custom|ExitGame
  (Game|QuitGame 0 "Quit" false))

(event Custom|SaveGame
  (bind _returnvalue (SaveGame|CreateSaveGameObject "/Game/Blueprints/Entrega_3/Save_Game.Save_Game_C"))
  (bind _output_get (Variables|Default|SetSaveGameRef _returnvalue))
  (Variables|/Game/Blueprints/Entrega_3/Save_Game.Save_Game_C|SetPlayerTransform _output_get (Transformation|GetActorTransform (Variables|Default|GetPlayer)))
  (Variables|/Game/Blueprints/Entrega_3/Save_Game.Save_Game_C|SetCoins _output_get (Variables|Default|GetCoins))
  (Variables|/Game/Blueprints/Entrega_3/Save_Game.Save_Game_C|SetKeys _output_get (Variables|Default|GetKeys))
  (Variables|/Game/Blueprints/Entrega_3/Save_Game.Save_Game_C|SetFirstDoorOpened _output_get (Variables|Default|GetFirstDoorOpened))
  (Variables|/Game/Blueprints/Entrega_3/Save_Game.Save_Game_C|SetFinalDoorOpened _output_get (Variables|Default|GetFinalDoorOpened))
  (SaveGame|SaveGametoSlot _returnvalue "SavedGame"))

(fn UseCoins
  (params (UsedCoins :type Integer))
  (Variables|Default|SetCoins (- (Variables|Default|GetCoins) UsedCoins)))