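; Automatic door trigger that lowers a referenced Door actor when the player enters and raises it back when the player leaves.
; BeginPlay caches the door's start position, a target Displacement units below it, and the first ThirdPersonCharacter found.
; Overlap events toggle Opening and Closing flags.
; Tick moves the door vertically at Speed scaled by delta time, without sweep, stopping once it passes either limit.
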(event EventBeginPlay
  (bind _door (Variables|Default|GetDoor))
  (bind _returnvalue (Transformation|GetActorLocation _door))
  ;[1 1 1] SET DOOR POSITIONS
  (Variables|Default|SetInitPos _returnvalue)
  (Variables|Default|SetFinalPos (- _returnvalue (* "0, 0,1.000000" (Variables|Default|GetDisplacement))))
  (bind _returnvalue_2 (Actor|GetActorOfClass "/Game/ThirdPersonBP/Blueprints/ThirdPersonCharacter.ThirdPersonCharacter_C"))
  (Variables|Default|SetPlayer _returnvalue_2))

(event Collision|EventActorBeginOverlap
  (params (OtherActor :type Actor%20Object%20Reference))
  ;[1 1 1] ENTER AND EXIT THE TRIGGER
  (if (== OtherActor (Variables|Default|GetPlayer))
    (Variables|Default|SetOpening true)
    (Variables|Default|SetClosing false)))

(event EventTick
  (params (DeltaSeconds :type Float%20%28single-precision%29))
  ;[1 1 1] OPEN DOOR
  (if (Variables|Default|GetOpening)
    (Transformation|AddActorWorldOffset (Variables|Default|GetDoor) (* "0, 0,-1.000000" (* (Utilities|Time|GetWorldDeltaSeconds) (Variables|Default|GetSpeed))))
    (if (<= (.Z (Math|Vector|BreakVector (Transformation|GetActorLocation (Variables|Default|GetDoor)))) (.Z (Math|Vector|BreakVector (Variables|Default|GetFinalPos))))
      (Variables|Default|SetOpening false))
    (else
      ;[1 1 1] CLOSE DOOR
      (if (Variables|Default|GetClosing)
        (Transformation|AddActorWorldOffset (Variables|Default|GetDoor) (* "0, 0,1.000000" (* (Utilities|Time|GetWorldDeltaSeconds) (Variables|Default|GetSpeed))))
        (if (>= (.Z (Math|Vector|BreakVector (Transformation|GetActorLocation (Variables|Default|GetDoor)))) (.Z (Math|Vector|BreakVector (Variables|Default|GetInitPos))))
          (Variables|Default|SetClosing false))))))

(event Collision|EventActorEndOverlap
  (params (OtherActor :type Actor%20Object%20Reference))
  ;[1 1 1] ENTER AND EXIT THE TRIGGER
  (if (== OtherActor (Variables|Default|GetPlayer))
    (Variables|Default|SetClosing true)
    (Variables|Default|SetOpening false)))

(fn ConstructionScript)