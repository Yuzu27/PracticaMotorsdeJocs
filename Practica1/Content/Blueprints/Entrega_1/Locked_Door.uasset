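; A door in an FPS game that the player unlocks by overlapping its box with enough coins or a key, as configured.
; A requirements widget shows the cost and animates on failure; success spends the currency and updates the HUD.
; Tick lowers the door, then destroys it, flags first or final door opened in the GameInstance, unlocks a checkpoint and saves.
; OpenedDoor removes the door instantly.
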(event OnComponentBeginOverlap(Box)
  (params (OverlappedComponent :type Primitive%20Component%20Object%20Reference) (OtherActor :type Actor%20Object%20Reference) (OtherComp :type Primitive%20Component%20Object%20Reference) (OtherBodyIndex :type Integer) (bFromSweep :type Boolean) (SweepResult :type Hit%20Result%20Structure%20%28by%20ref%29))
  (bind _returnvalue (Game|GetGameInstance))
  (bind _returnvalue_2 (Game|GetGameInstance))
  (bind _asfpsgame_instance (Utilities|Casting|CastToFPSGameInstance _returnvalue))
  (bind _asfpsgame_instance_2 (Utilities|Casting|CastToFPSGameInstance _returnvalue_2))
  (if (and (Variables|Default|GetClosed) (== OtherActor (Variables|/Game/Blueprints/Entrega_2/FPSGameInstance.FPSGameInstance_C|GetPlayer (.AsFPSGame%20Instance (Utilities|Casting|CastToFPSGameInstance (Game|GetGameInstance))))))
    (if (Variables|Default|GetLockedByCoins)
      (if (>= (Variables|/Game/Blueprints/Entrega_2/FPSGameInstance.FPSGameInstance_C|GetCoins (.AsFPSGame%20Instance (Utilities|Casting|CastToFPSGameInstance (Game|GetGameInstance)))) (Variables|Default|GetCoinsNeeded))
        (Audio|PlaySoundatLocation "/Game/Assets/Sounds/DoorSound_Cue.DoorSound_Cue" (Variables|/Script/Engine.SceneComponent|GetRelativeLocation (Variables|Default|GetDoor)) "0, 0, 0" 1.0 1.0 0.0 0 0 0)
        (Variables|Default|SetOpening true)
        (Default|UseCoins _asfpsgame_instance_2 (Variables|Default|GetCoinsNeeded))
        (Default|UpdateCoins (Variables|/Game/Blueprints/Entrega_2/HUD/HUD_Controller.HUD_Controller_C|GetUI (Variables|/Game/Blueprints/Entrega_2/FPSGameInstance.FPSGameInstance_C|GetHUDController _asfpsgame_instance_2)))
        (Variables|Default|SetClosed false :!label _label)
        (Components|DestroyComponent (Variables|Default|GetRequirements))
        (else
          (Default|RequirementsAnimation (.AsDoor%20Requirements (Utilities|Casting|CastToDoor_Requirements (UserInterface|GetUserWidgetObject (Variables|Default|GetRequirements)))) :!label _label_2)))
      (elif (>= (Variables|/Game/Blueprints/Entrega_2/FPSGameInstance.FPSGameInstance_C|GetKeys (.AsFPSGame%20Instance (Utilities|Casting|CastToFPSGameInstance (Game|GetGameInstance)))) 1)
        (Audio|PlaySoundatLocation "/Game/Assets/Sounds/DoorSound_Cue.DoorSound_Cue" (Variables|/Script/Engine.SceneComponent|GetRelativeLocation (Variables|Default|GetDoor)) "0, 0, 0" 1.0 1.0 0.0 0 0 0)
        (Variables|Default|SetOpening true)
        (Default|UseKey _asfpsgame_instance)
        (Default|UpdateKeys (Variables|/Game/Blueprints/Entrega_2/HUD/HUD_Controller.HUD_Controller_C|GetUI (Variables|/Game/Blueprints/Entrega_2/FPSGameInstance.FPSGameInstance_C|GetHUDController _asfpsgame_instance)))
        (goto _label)
        (else
          (goto _label_2))))))

(event Custom|OpenedDoor
  (Variables|Default|SetClosed false)
  (Components|DestroyComponent (Variables|Default|GetDoor)))

(event EventBeginPlay
  (bind _door (Variables|Default|GetDoor))
  (bind _returnvalue (Transformation|GetWorldLocation _door))
  ;[1 1 1] SET DOOR POSITIONS
  (Variables|Default|SetInitPos _returnvalue)
  (Variables|Default|SetFinalPos (- _returnvalue (* "0, 0,1.000000" (Variables|Default|GetDisplacement))))
  (Default|UpdateDoorRequirements (.AsDoor%20Requirements (Utilities|Casting|CastToDoor_Requirements (UserInterface|GetUserWidgetObject (Variables|Default|GetRequirements)))) (Variables|Default|GetLockedByCoins) (Variables|Default|GetCoinsNeeded)))

(event EventTick
  (params (DeltaSeconds :type Float%20%28single-precision%29))
  (bind _returnvalue (Game|GetGameInstance))
  (bind _returnvalue_2 (Game|GetGameInstance))
  (bind _asfpsgame_instance (Utilities|Casting|CastToFPSGameInstance _returnvalue_2))
  (bind _asfpsgame_instance_2 (Utilities|Casting|CastToFPSGameInstance _returnvalue))
  ;[1 1 1] OPEN DOOR
  (if (Variables|Default|GetOpening)
    (Transformation|AddWorldOffset (Variables|Default|GetDoor) (* "0, 0,-1.000000" (* (Utilities|Time|GetWorldDeltaSeconds) (Variables|Default|GetSpeed))) false false)
    (if (<= (.Z (Math|Vector|BreakVector (Transformation|GetWorldLocation (Variables|Default|GetDoor)))) (.Z (Math|Vector|BreakVector (Variables|Default|GetFinalPos))))
      (Variables|Default|SetOpening false)
      (Components|DestroyComponent (Variables|Default|GetDoor))
      (if (Variables|/Game/Blueprints/Entrega_2/FPSGameInstance.FPSGameInstance_C|GetFirstDoorOpened _asfpsgame_instance_2)
        (Variables|/Game/Blueprints/Entrega_2/FPSGameInstance.FPSGameInstance_C|SetFinalDoorOpened _asfpsgame_instance_2 true)
        (else
          (Variables|/Game/Blueprints/Entrega_2/FPSGameInstance.FPSGameInstance_C|SetFirstDoorOpened _asfpsgame_instance_2 true)))
      (Default|CheckpointUnlocked (Variables|/Game/Blueprints/Entrega_2/FPSGameInstance.FPSGameInstance_C|GetHUDController _asfpsgame_instance))
      (Default|SaveGame _asfpsgame_instance)
      (Audio|SpawnSound2D "/Game/Assets/Sounds/ManualSave.ManualSave" 1.0 1.0 0.0 0))))

(fn ConstructionScript)

(fn DoorSound+)