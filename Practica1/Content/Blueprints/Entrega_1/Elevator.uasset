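; Elevator platform that rises while the player stands within its Sphere trigger and descends when they leave.
; BeginPlay stores the start position and a top position offset upward by Displacement.
; Overlap events play a sound for any actor, but set the up or down flags only for the player held in FPSGameInstance.
; Tick moves the actor vertically at Speed without sweep, stopping once it reaches either limit.
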(event OnComponentBeginOverlap(Sphere)
  (params (OverlappedComponent :type Primitive%20Component%20Object%20Reference) (OtherActor :type Actor%20Object%20Reference) (OtherComp :type Primitive%20Component%20Object%20Reference) (OtherBodyIndex :type Integer) (bFromSweep :type Boolean) (SweepResult :type Hit%20Result%20Structure%20%28by%20ref%29))
  (Audio|PlaySoundatLocation "/Game/Assets/Sounds/ElevatorSound_Cue.ElevatorSound_Cue" (Transformation|GetWorldLocation (Variables|Default|GetSphere)) "0, 0, 0" 1.0 1.0 0.0 0 0 0)
  ;[1 1 1] ENTER THE PLATFORM
  (if (== OtherActor (Variables|/Game/Blueprints/Entrega_2/FPSGameInstance.FPSGameInstance_C|GetPlayer (.AsFPSGame%20Instance (Utilities|Casting|CastToFPSGameInstance (Game|GetGameInstance)))))
    (Variables|Default|SetGoingUp true)
    (Variables|Default|SetGoingDown false)))

(event OnComponentEndOverlap(Sphere)
  (params (OverlappedComponent :type Primitive%20Component%20Object%20Reference) (OtherActor :type Actor%20Object%20Reference) (OtherComp :type Primitive%20Component%20Object%20Reference) (OtherBodyIndex :type Integer))
  (Audio|PlaySoundatLocation "/Game/Assets/Sounds/ElevatorSound_Cue.ElevatorSound_Cue" (Transformation|GetWorldLocation (Variables|Default|GetSphere)) "0, 0, 0" 1.0 1.0 0.0 0 0 0)
  ;[1 1 1] EXIT THE PLATFORM
  (if (== OtherActor (Variables|/Game/Blueprints/Entrega_2/FPSGameInstance.FPSGameInstance_C|GetPlayer (.AsFPSGame%20Instance (Utilities|Casting|CastToFPSGameInstance (Game|GetGameInstance)))))
    (Variables|Default|SetGoingDown true)
    (Variables|Default|SetGoingUp false)))

(event EventBeginPlay
  (bind _returnvalue (Transformation|GetActorLocation))
  ;[1 1 1] SET PLATFORM POSITIONS
  (Variables|Default|SetInitPos _returnvalue)
  (Variables|Default|SetFinalPos (+ _returnvalue (* "0, 0,1.000000" (Variables|Default|GetDisplacement)))))

(event EventTick
  (params (DeltaSeconds :type Float%20%28single-precision%29))
  ;[1 1 1] PLATFORM GOING UP
  (if (Variables|Default|GetGoingUp)
    (Transformation|AddActorWorldOffset (* "0, 0,1.000000" (* (Utilities|Time|GetWorldDeltaSeconds) (Variables|Default|GetSpeed))))
    (if (>= (.Z (Math|Vector|BreakVector (Transformation|GetActorLocation))) (.Z (Math|Vector|BreakVector (Variables|Default|GetFinalPos))))
      (Variables|Default|SetGoingUp false))
    (else
      ;[1 1 1] PLATFOMR GOING DOWN
      (if (Variables|Default|GetGoingDown)
        (Transformation|AddActorWorldOffset (* "0, 0,-1.000000" (* (Utilities|Time|GetWorldDeltaSeconds) (Variables|Default|GetSpeed))))
        (if (<= (.Z (Math|Vector|BreakVector (Transformation|GetActorLocation))) (.Z (Math|Vector|BreakVector (Variables|Default|GetInitPos))))
          (Variables|Default|SetGoingDown false))))))

(fn ConstructionScript)