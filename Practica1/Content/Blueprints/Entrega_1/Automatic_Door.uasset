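; Automatic door that sinks downward when the player enters its trigger box and rises back when they leave.
; BeginPlay caches the closed position and an open position offset down by Displacement.
; Box overlaps, filtered to the GameInstance's Player reference, set Opening/Closing flags and play a sound at the door's relative location.
; Tick moves the door at Speed scaled by delta time, without sweep, until it passes either limit.
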(event OnComponentBeginOverlap(Box)
  (params (OverlappedComponent :type Primitive%20Component%20Object%20Reference) (OtherActor :type Actor%20Object%20Reference) (OtherComp :type Primitive%20Component%20Object%20Reference) (OtherBodyIndex :type Integer) (bFromSweep :type Boolean) (SweepResult :type Hit%20Result%20Structure%20%28by%20ref%29))
  ;[1 1 1] ENTER AND EXIT THE TRIGGER
  (if (== OtherActor (Variables|/Game/Blueprints/Entrega_2/FPSGameInstance.FPSGameInstance_C|GetPlayer (.AsFPSGame%20Instance (Utilities|Casting|CastToFPSGameInstance (Game|GetGameInstance)))))
    (CallFunction|PlayDoorSound)
    (Variables|Default|SetOpening true)
    (Variables|Default|SetClosing false)))

(event OnComponentEndOverlap(Box)
  (params (OverlappedComponent :type Primitive%20Component%20Object%20Reference) (OtherActor :type Actor%20Object%20Reference) (OtherComp :type Primitive%20Component%20Object%20Reference) (OtherBodyIndex :type Integer))
  ;[1 1 1] ENTER AND EXIT THE TRIGGER
  (if (== OtherActor (Variables|/Game/Blueprints/Entrega_2/FPSGameInstance.FPSGameInstance_C|GetPlayer (.AsFPSGame%20Instance (Utilities|Casting|CastToFPSGameInstance (Game|GetGameInstance)))))
    (CallFunction|PlayDoorSound)
    (Variables|Default|SetClosing true)
    (Variables|Default|SetOpening false)))

(event EventBeginPlay
  (bind _door (Variables|Default|GetDoor))
  (bind _returnvalue (Transformation|GetWorldLocation _door))
  ;[1 1 1] SET DOOR POSITIONS
  (Variables|Default|SetInitPos _returnvalue)
  (Variables|Default|SetFinalPos (- _returnvalue (* "0, 0,1.000000" (Variables|Default|GetDisplacement)))))

(event EventTick
  (params (DeltaSeconds :type Float%20%28single-precision%29))
  ;[1 1 1] OPEN DOOR
  (if (Variables|Default|GetOpening)
    (Transformation|AddWorldOffset (Variables|Default|GetDoor) (* "0, 0,-1.000000" (* (Utilities|Time|GetWorldDeltaSeconds) (Variables|Default|GetSpeed))) false false)
    (if (<= (.Z (Math|Vector|BreakVector (Transformation|GetWorldLocation (Variables|Default|GetDoor)))) (.Z (Math|Vector|BreakVector (Variables|Default|GetFinalPos))))
      (Variables|Default|SetOpening false))
    (else
      ;[1 1 1] CLOSE DOOR
      (if (Variables|Default|GetClosing)
        (Transformation|AddWorldOffset (Variables|Default|GetDoor) (* "0, 0,1.000000" (* (Utilities|Time|GetWorldDeltaSeconds) (Variables|Default|GetSpeed))) false false)
        (if (>= (.Z (Math|Vector|BreakVector (Transformation|GetWorldLocation (Variables|Default|GetDoor)))) (.Z (Math|Vector|BreakVector (Variables|Default|GetInitPos))))
          (Variables|Default|SetClosing false))))))

(fn ConstructionScript)

(fn PlayDoorSound
  (Audio|PlaySoundatLocation "/Game/Blueprints/Entrega_3/SoundEffects/AutomaticDoor_Cue.AutomaticDoor_Cue" (Variables|/Script/Engine.SceneComponent|GetRelativeLocation (Variables|Default|GetDoor)) "0, 0, 0" 1.0 1.0 0.0 0 0 0))