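; A locked door actor that opens when the player overlaps it with enough coins or a key, chosen by a LockedByCoins flag.
; On success it spends the coins or key through the FPS game instance and refreshes the HUD, otherwise it prints what is missing.
; Tick slides the door downward at a set speed and destroys the actor once it passes its displaced end position.
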(event EventBeginPlay
  (bind _door (Variables|Default|GetDoor))
  (bind _returnvalue (Transformation|GetActorLocation _door))
  ;[1 1 1] SET DOOR POSITIONS
  (Variables|Default|SetInitPos _returnvalue)
  (Variables|Default|SetFinalPos (- _returnvalue (* "0, 0,1.000000" (Variables|Default|GetDisplacement)))))

(event Collision|EventActorBeginOverlap
  (params (OtherActor :type Actor%20Object%20Reference))
  (bind _returnvalue (Game|GetGameInstance))
  (bind _returnvalue_2 (Game|GetGameInstance))
  (bind _returnvalue_3 (Game|GetGameInstance))
  (bind _coinsneeded (Variables|Default|GetCoinsNeeded))
  (bind _asfpsgame_instance (Utilities|Casting|CastToFPSGameInstance _returnvalue_3))
  (bind _asfpsgame_instance_2 (Utilities|Casting|CastToFPSGameInstance _returnvalue))
  (bind _asfpsgame_instance_3 (Utilities|Casting|CastToFPSGameInstance _returnvalue_2))
  (bind _coins (Variables|/Game/Blueprints/Entrega_2/FPSGameInstance.FPSGameInstance_C|GetCoins _asfpsgame_instance_2))
  (if (== OtherActor (Variables|/Game/Blueprints/Entrega_2/FPSGameInstance.FPSGameInstance_C|GetPlayer (.AsFPSGame%20Instance (Utilities|Casting|CastToFPSGameInstance (Game|GetGameInstance)))))
    (if (Variables|Default|GetLockedByCoins)
      (if (>= _coins _coinsneeded)
        (Variables|Default|SetOpening true)
        (Default|UseCoins _asfpsgame_instance_3 (Variables|Default|GetCoinsNeeded))
        (Default|UpdateCoins (Variables|/Game/Blueprints/Entrega_2/HUD/HUD_Controller.HUD_Controller_C|GetUI (Variables|/Game/Blueprints/Entrega_2/FPSGameInstance.FPSGameInstance_C|GetHUDController _asfpsgame_instance_3)))
        (else
          (Development|PrintString (Utilities|String|Append "YOU NEED " (Utilities|String|ToString(Integer) (- _coinsneeded _coins)) " MORE COINS"))))
      (elif (>= (Variables|/Game/Blueprints/Entrega_2/FPSGameInstance.FPSGameInstance_C|GetKeys (.AsFPSGame%20Instance (Utilities|Casting|CastToFPSGameInstance (Game|GetGameInstance)))) 1)
        (Variables|Default|SetOpening true)
        (Default|UseKey _asfpsgame_instance)
        (Default|UpdateKeys (Variables|/Game/Blueprints/Entrega_2/HUD/HUD_Controller.HUD_Controller_C|GetUI (Variables|/Game/Blueprints/Entrega_2/FPSGameInstance.FPSGameInstance_C|GetHUDController _asfpsgame_instance)))
        (else
          (Development|PrintString "YOU NEED THE KEY"))))))

(event EventTick
  (params (DeltaSeconds :type Float%20%28single-precision%29))
  ;[1 1 1] OPEN DOOR
  (if (Variables|Default|GetOpening)
    (Transformation|AddActorWorldOffset (Variables|Default|GetDoor) (* "0, 0,-1.000000" (* (Utilities|Time|GetWorldDeltaSeconds) (Variables|Default|GetSpeed))))
    (if (<= (.Z (Math|Vector|BreakVector (Transformation|GetActorLocation (Variables|Default|GetDoor)))) (.Z (Math|Vector|BreakVector (Variables|Default|GetFinalPos))))
      (Actor|DestroyActor))))

(fn ConstructionScript)