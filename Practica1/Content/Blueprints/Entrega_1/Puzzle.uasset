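; Light-colour puzzle actor that opens a chest and spawns a key when three lights show the right colours.
; Every Tick, it compares the left, centre and right light colours against their target colour variables.
; On the first full match, a Solved flag blocks repeats, a Key spawns at the puzzle actor's transform, and the closed chest actor is swapped for the open one, hidden since BeginPlay.
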(event EventTick
  (params (DeltaSeconds :type Float%20%28single-precision%29))
  (if (Math|Boolean|ANDBoolean (== (Rendering|Components|Light|GetLightColor (Variables|/Script/Engine.Light|GetLightComponent (Variables|Default|GetLeftLight))) (Math|Conversions|ToLinearColor(Color) (Variables|Default|GetLeftColor))) (== (Rendering|Components|Light|GetLightColor (Variables|/Script/Engine.Light|GetLightComponent (Variables|Default|GetCenterLight))) (Math|Conversions|ToLinearColor(Color) (Variables|Default|GetCenterColor))) (== (Rendering|Components|Light|GetLightColor (Variables|/Script/Engine.Light|GetLightComponent (Variables|Default|GetRightLight))) (Math|Conversions|ToLinearColor(Color) (Variables|Default|GetRightColor))))
    (if (not (Variables|Default|GetSolved))
      (Variables|Default|SetSolved true)
      (Game|SpawnActorfromClass "/Game/Blueprints/Entrega_1/Key.Key_C" (Transformation|GetActorTransform) "Undefined" 0 0)
      (Rendering|SetActorHiddenInGame (Variables|Default|GetChestOpened) false)
      (Rendering|SetActorHiddenInGame (Variables|Default|GetChestClosed) true))))

(event EventBeginPlay
  (Rendering|SetActorHiddenInGame (Variables|Default|GetChestOpened) true))

(fn ConstructionScript)