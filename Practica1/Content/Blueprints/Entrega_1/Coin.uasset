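; Collectible coin actor that the player picks up by touching it.
; When its Box collider overlaps the player stored in FPSGameInstance, it calls CollectCoin on the game instance and refreshes the coin count through the HUD controller's UI widget.
; It then destroys itself.
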(event OnComponentBeginOverlap(Box)
  (params (OverlappedComponent :type Primitive%20Component%20Object%20Reference) (OtherActor :type Actor%20Object%20Reference) (OtherComp :type Primitive%20Component%20Object%20Reference) (OtherBodyIndex :type Integer) (bFromSweep :type Boolean) (SweepResult :type Hit%20Result%20Structure%20%28by%20ref%29))
  (bind _returnvalue (Game|GetGameInstance))
  (bind _asfpsgame_instance (Utilities|Casting|CastToFPSGameInstance _returnvalue))
  (if (== OtherActor (Variables|/Game/Blueprints/Entrega_2/FPSGameInstance.FPSGameInstance_C|GetPlayer (.AsFPSGame%20Instance (Utilities|Casting|CastToFPSGameInstance (Game|GetGameInstance)))))
    (Default|CollectCoin _asfpsgame_instance)
    (Default|UpdateCoins (Variables|/Game/Blueprints/Entrega_2/HUD/HUD_Controller.HUD_Controller_C|GetUI (Variables|/Game/Blueprints/Entrega_2/FPSGameInstance.FPSGameInstance_C|GetHUDController _asfpsgame_instance)))
    (Actor|DestroyActor)))

(fn ConstructionScript)