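; LockedDoor is a blueprint for a door that the ThirdPersonCharacter unlocks with either coins or a key, chosen by the LockedByCoins flag.
; On overlap it checks the player's Coins or Keys, then spends them and starts opening, or prints what is missing.
; While opening, Tick slides the referenced Door actor downward at Speed and destroys the LockedDoor actor once the door has dropped by Displacement.
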(event EventBeginPlay
  (bind _door (Variables|Default|GetDoor))
  (bind _returnvalue (Transformation|GetActorLocation _door))
  ;[1 1 1] SET DOOR POSITIONS
  (Variables|Default|SetInitPos _returnvalue)
  (Variables|Default|SetFinalPos (- _returnvalue (* "0, 0,1.000000" (Variables|Default|GetDisplacement))))
  (bind _returnvalue_2 (Actor|GetActorOfClass "/Game/ThirdPersonBP/Blueprints/ThirdPersonCharacter.ThirdPersonCharacter_C"))
  (Variables|Default|SetPlayer _returnvalue_2))

(event Collision|EventActorBeginOverlap
  (params (OtherActor :type Actor%20Object%20Reference))
  (bind _player (Variables|Default|GetPlayer))
  (bind _coinsneeded (Variables|Default|GetCoinsNeeded))
  (bind _coins (Variables|/Game/ThirdPersonBP/Blueprints/ThirdPersonCharacter.ThirdPersonCharacter_C|GetCoins _player))
  (if (== OtherActor (Variables|Default|GetPlayer))
    (if (Variables|Default|GetLockedByCoins)
      (if (>= _coins _coinsneeded)
        (Variables|Default|SetOpening true)
        (Default|CoinsUsed (Variables|Default|GetPlayer) (Variables|Default|GetCoinsNeeded))
        (else
          (Development|PrintString (Utilities|String|Append "YOU NEED " (Utilities|String|ToString(Integer) (- _coinsneeded _coins)) " MORE COINS"))))
      (elif (>= (Variables|/Game/ThirdPersonBP/Blueprints/ThirdPersonCharacter.ThirdPersonCharacter_C|GetKeys (Variables|Default|GetPlayer)) 1)
        (Variables|Default|SetOpening true)
        (Default|KeyUsed (Variables|Default|GetPlayer))
        (else
          (Development|PrintString "YOU NEED THE KEY"))))))

(event EventTick
  (params (DeltaSeconds :type Float%20%28single-precision%29))
  ;[1 1 1] OPEN DOOR
  (if (Variables|Default|GetOpening)
    (Transformation|AddActorWorldOffset (Variables|Default|GetDoor) (* "0, 0,-1.000000" (* (Utilities|Time|GetWorldDeltaSeconds) (Variables|Default|GetSpeed))))
    (if (<= (.Z (Math|Vector|BreakVector (Transformation|GetActorLocation (Variables|Default|GetDoor)))) (.Z (Math|Vector|BreakVector (Variables|Default|GetFinalPos))))
      (Actor|DestroyActor))))

(fn ConstructionScript)