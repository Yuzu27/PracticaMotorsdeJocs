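; PuzzleButton is an overlap-triggered puzzle button that cycles a linked light through red, yellow, blue and green.
; On BeginPlay it builds the color array and caches the ThirdPersonCharacter as the player.
; When that player enters the Sphere and the referenced Puzzle is unsolved, it applies the current color to the Light, then advances the index with wraparound.
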(event OnComponentBeginOverlap(Sphere)
  (params (OverlappedComponent :type Primitive%20Component%20Object%20Reference) (OtherActor :type Actor%20Object%20Reference) (OtherComp :type Primitive%20Component%20Object%20Reference) (OtherBodyIndex :type Integer) (bFromSweep :type Boolean) (SweepResult :type Hit%20Result%20Structure%20%28by%20ref%29))
  (if (and (== OtherActor (Variables|Default|GetPlayer)) (not (Variables|/Game/Blueprints/Puzzle.Puzzle_C|GetSolved (Variables|Default|GetPuzzle))))
    (Rendering|Components|Light|SetLightColor (Variables|/Script/Engine.Light|GetLightComponent (Variables|Default|GetLight)) (Math|Conversions|ToLinearColor(Color) (Utilities|Array|Get(acopy) (Variables|Default|GetColors) (Variables|Default|GetCurrentColorIdx))) true)
    (if (>= (Variables|Default|GetCurrentColorIdx) (- (Utilities|Array|Length (Variables|Default|GetColors)) 1))
      (Variables|Default|SetCurrentColorIdx 0)
      (else
        (Variables|Default|SetCurrentColorIdx (+ (Variables|Default|GetCurrentColorIdx) 1))))))

(event EventBeginPlay
  (Variables|Default|SetColors (Utilities|Array|MakeArray (Variables|Default|GetRed) (Variables|Default|GetYellow) (Variables|Default|GetBlue) (Variables|Default|GetGreen)))
  (bind _returnvalue (Actor|GetActorOfClass "/Game/ThirdPersonBP/Blueprints/ThirdPersonCharacter.ThirdPersonCharacter_C"))
  (Variables|Default|SetPlayer _returnvalue))

(fn ConstructionScript)